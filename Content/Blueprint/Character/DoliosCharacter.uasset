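; DoliosCharacter is the player character, with tank-style turn and forward-only movement, pistol aiming and firing flags.
; BeginPlay creates the HUD; Tick refreshes info text and life bar, opening a paused Game Over screen when Vida drops below zero.
; Aiming blocks walking, uses a sphere trace to snap yaw toward an AI_Character, and moves the pistol between sockets after delays.
; Start opens an animated pause menu.
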(event EventTick
  (params (DeltaSeconds :type Float%20%28single-precision%29))
  ;[1 1 1] Hud
  (Rendering|Components|TextRender|SetText (Variables|/Game/Blueprint/Widgets/GameplayWid.GameplayWid_C|GetInformacoes (stale EventBeginPlay _returnvalue)) (Utilities|Text|ToText(String) (Variables|Default|GetSinformacoes)))
  (Widget|SetVisibility (Variables|/Game/Blueprint/Widgets/GameplayWid.GameplayWid_C|GetInformacoes (stale EventBeginPlay _returnvalue)) (Variables|Default|GetVisibilidade))
  (Progress|SetPercent (Variables|/Game/Blueprint/Widgets/GameplayWid.GameplayWid_C|GetLifeBar (stale EventBeginPlay _returnvalue)) (/ (Math|Conversions|ToFloat(Integer) (Variables|Default|GetVida)) 1e+02))
  (if (< (Variables|Default|GetVida) 0)
    (bind _returnvalue (UserInterface|CreateWidget "/Game/Blueprint/Widgets/GameOver.GameOver_C"))
    (bind _output_get (Variables|Default|SetMorte _returnvalue))
    (UserInterface|Viewport|AddtoViewport _output_get 0)
    (Variables|/Script/Engine.PlayerController|SetbShowMouseCursor (Game|GetPlayerController 0) true)
    (Game|SetGamePaused true)))

(event EventBeginPlay
  ;[1 1 1] Hud
  (bind _returnvalue (UserInterface|CreateWidget "/Game/Blueprint/Widgets/GameplayWid.GameplayWid_C"))
  (UserInterface|Viewport|AddtoViewport _returnvalue 0)
  (Game|SetGamePaused false))

(event Input|ActionEvents|InputActionStart
  (params (Key :type Key%20Structure :default "AnyKey"))
  ;[1 1 1] Input
  (:Pressed
    (bind _returnvalue (UserInterface|CreateWidget "/Game/Blueprint/Widgets/Pause.Pause_C"))
    (Variables|Default|SetPauseWidget _returnvalue)
    (UserInterface|Viewport|AddtoViewport (Variables|Default|GetPauseWidget) 0)
    (UserInterface|Animation|PlayAnimation (Variables|Default|GetPauseWidget) (Variables|/Game/Blueprint/Widgets/Pause.Pause_C|GetAnimaçãoPainel (Variables|Default|GetPauseWidget)) 0.0 1 "Forward")
    (UserInterface|Animation|PlayAnimation (Variables|Default|GetPauseWidget) (Variables|/Game/Blueprint/Widgets/Pause.Pause_C|GetAnimaçãoSimbolo (Variables|Default|GetPauseWidget)) 0.0 0 "Forward")
    (UserInterface|Animation|PlayAnimation (Variables|Default|GetPauseWidget) (Variables|/Game/Blueprint/Widgets/Pause.Pause_C|GetAnimaçãoListra (Variables|Default|GetPauseWidget)) 0.0 0 "Forward")
    (Variables|/Script/Engine.PlayerController|SetbShowMouseCursor (Game|GetPlayerController 0) true)
    (Game|SetGamePaused true)))

(event Input|ActionEvents|InputActionMirar
  (params (Key :type Key%20Structure :default "AnyKey"))
  (bind _returnvalue (Transformation|GetActorLocation))
  ;[1 1 1] Input
  (:Pressed
    (if (not (Variables|Default|GetPrecionouMirar))
      (Variables|Default|SetPrecionouMirar true)
      (Variables|Default|SetSacouArma true)
      (bind _outhit (Collision|SphereTraceForObjects _returnvalue (+ _returnvalue "0, 0,0.100000") 1e+03 (Variables|Default|GetObjectType) false 0 "None"))
      (if (!= (.HitComponent (Collision|BreakHitResult _outhit)) 0)
        (bind _asai_character (Utilities|Casting|CastToAI_Character (Components|GetOwner (.HitComponent (Collision|BreakHitResult _outhit)))))
        (if (== (.HitComponent (Collision|BreakHitResult _outhit)) (Variables|/Script/Engine.Character|GetCapsuleComponent _asai_character))
          (Pawn|SetControlRotation (Pawn|GetController) (Math|Rotator|MakeRotator 0.0 0.0 (.Yaw (Math|Rotator|BreakRotator (Math|Rotator|FindLookatRotation (Transformation|GetActorLocation) (Transformation|GetActorLocation (Components|GetOwner (.HitComponent (Collision|BreakHitResult _outhit)))))))))
          (Utilities|FlowControl|Delay 0.4 :!label _label)
          (Transformation|AttachComponentToComponent (Variables|Default|GetPistola) (Variables|Character|GetMesh) "Armado" "KeepRelative" "KeepRelative" "KeepRelative" true))
        (else
          (goto _label)))))
  (:Released
    (if (Variables|Default|GetPrecionouMirar)
      (Variables|Default|SetSacouArma false)
      (Utilities|FlowControl|Delay 0.8)
      (Transformation|AttachComponentToComponent (Variables|Default|GetPistola) (Variables|Character|GetMesh) "Arma" "KeepRelative" "KeepRelative" "KeepRelative" true)
      (Utilities|FlowControl|Delay 1.0)
      (Variables|Default|SetPrecionouMirar false))))

(event Input|ActionEvents|InputActionAtirar
  (params (Key :type Key%20Structure :default "AnyKey"))
  ;[1 1 1] Input
  (:Pressed
    (if (Variables|Default|GetPrecionouMirar)
      (if (not (Variables|Default|GetPrecionarTiro))
        (Variables|Default|SetPrecionarTiro true)
        (Variables|Default|SetAtirou true))))
  (:Released
    (if (Variables|Default|GetPrecionouMirar)
      (Variables|Default|SetPrecionarTiro false)
      (Variables|Default|SetAtirou false))))

(event Input|AxisEvents|InputAxisHorizontal
  (params (AxisValue :type Float%20%28single-precision%29))
  ;[1 1 1] Input
  (Pawn|Input|AddControllerYawInput (* AxisValue (Variables|Default|GetVelocidadeRotacao))))

(event Input|AxisEvents|InputAxisVertical
  (params (AxisValue :type Float%20%28single-precision%29))
  ;[1 1 1] Input
  (if (>= AxisValue 0.0)
    (if (not (Variables|Default|GetPrecionouMirar))
      (Pawn|Input|AddMovementInput (Math|Vector|GetForwardVector (Math|Rotator|MakeRotator 0.0 0.0 (.Yaw (Math|Rotator|BreakRotator (Pawn|GetControlRotation :!class /Script/Engine.Pawn))))) AxisValue false))))

(fn ConstructionScript)