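; DoliosCharacter is the player character, with axis-driven turning and forward/back movement through local offsets without sweep, plus a pause menu.
; The camera detaches at start, then each Tick interpolates toward the CameraPosicao anchor and looks at ProtoPersonagem.
; The Pause input creates an animated widget, shows the cursor and sets a flag blocking movement and camera updates.
; Tick polls the widget's SairPause flag, reverses the animation, then hides it and unpauses after a delay.
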(event Collision|EventActorBeginOverlap
  (params (OtherActor :type Actor%20Object%20Reference)))

(event EventTick
  (params (DeltaSeconds :type Float%20%28single-precision%29))
  (bind _pausewidget (Variables|Default|GetPauseWidget))
  ;[1 1 1] CameraControl
  (if (Variables|Default|GetPause)
    (if (Variables|/Game/Blueprint/Pause.Pause_C|GetSairPause _pausewidget)
      (Variables|/Game/Blueprint/Pause.Pause_C|SetSairPause _pausewidget false)
      (UserInterface|Animation|PlayAnimation _pausewidget (Variables|/Game/Blueprint/Pause.Pause_C|GetAnimaçãoPainel _pausewidget) 0.0 1 "Reverse")
      (Utilities|FlowControl|Delay 3.0)
      (Widget|SetVisibility _pausewidget "Hidden")
      (Variables|Default|SetPause false))
    (else
      (Transformation|SetWorldLocationAndRotation (Variables|Default|GetCamera) (Math|Interpolation|VInterpTo (Transformation|GetWorldLocation (Variables|Default|GetCamera)) (Transformation|GetWorldLocation (Variables|Default|GetCameraPosicao)) DeltaSeconds (Variables|Default|GetVelocidadeSeguir)) (Math|Rotator|FindLookatRotation (Transformation|GetWorldLocation (Variables|Default|GetCamera)) (Transformation|GetWorldLocation (Variables|Default|GetProtoPersonagem))) false false))))

(event EventBeginPlay
  ;[1 1 1] CameraControl
  (Transformation|DetachFromComponent (Variables|Default|GetCamera) "KeepRelative" "KeepRelative" "KeepRelative" true))

(event Input|ActionEvents|InputActionPause
  (params (Key :type Key%20Structure :default "AnyKey"))
  (:Pressed
    (if (not (Variables|Default|GetPause))
      (bind _returnvalue (UserInterface|CreateWidget "/Game/Blueprint/Pause.Pause_C"))
      (Variables|Default|SetPauseWidget _returnvalue)
      (Variables|Default|SetPause true)
      (UserInterface|Viewport|AddtoViewport (Variables|Default|GetPauseWidget) 0)
      (UserInterface|Animation|PlayAnimation (Variables|Default|GetPauseWidget) (Variables|/Game/Blueprint/Pause.Pause_C|GetAnimaçãoPainel (Variables|Default|GetPauseWidget)) 0.0 1 "Forward")
      (Variables|/Script/Engine.PlayerController|SetbShowMouseCursor (Game|GetPlayerController 0) true))))

(event Input|AxisEvents|InputAxisHorizontal
  (params (AxisValue :type Float%20%28single-precision%29))
  ;[1 1 1] Input
  (if (not (Variables|Default|GetPause))
    (Transformation|AddActorLocalRotation (Math|Rotator|MakeRotator 0.0 0.0 (* AxisValue (Variables|Default|GetVelocidadeRotacao))) false false)))

(event Input|AxisEvents|InputAxisVertical
  (params (AxisValue :type Float%20%28single-precision%29))
  ;[1 1 1] Input
  (if (not (Variables|Default|GetPause))
    (Transformation|AddActorLocalOffset (Math|Vector|MakeVector (* AxisValue (Variables|Default|GetVelocidade)) 0.0 0.0) false false)))

(fn ConstructionScript)