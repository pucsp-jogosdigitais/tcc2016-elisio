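; Interactive lever actor that rotates a bridge (Ponte) when E is pressed within its trigger area.
; Begin and end overlap on Cube enable and disable player 0's input on the actor, without checking which actor overlaps.
; E instantly sets the bridge's roll to 90 degrees and raises PodeRodar, which is never cleared.
; While that flag is set, Tick uses RInterpTo to ease the lever (Alavanca) toward a fixed world rotation.
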(event OnComponentBeginOverlap(Cube)
  (params (OverlappedComponent :type Primitive%20Component%20Object%20Reference) (OtherActor :type Actor%20Object%20Reference) (OtherComp :type Primitive%20Component%20Object%20Reference) (OtherBodyIndex :type Integer) (bFromSweep :type Boolean) (SweepResult :type Hit%20Result%20Structure%20%28by%20ref%29))
  (Input|EnableInput (Game|GetPlayerController 0)))

(event OnComponentEndOverlap(Cube)
  (params (OverlappedComponent :type Primitive%20Component%20Object%20Reference) (OtherActor :type Actor%20Object%20Reference) (OtherComp :type Primitive%20Component%20Object%20Reference) (OtherBodyIndex :type Integer))
  (Input|DisableInput (Game|GetPlayerController 0)))

(event EventTick
  (params (DeltaSeconds :type Float%20%28single-precision%29))
  (Variables|Default|SetDelta DeltaSeconds)
  (if (Variables|Default|GetPodeRodar)
    (Transformation|SetWorldRotation (Variables|Default|GetAlavanca) (Math|Interpolation|RInterpTo (Transformation|GetWorldRotation (Variables|Default|GetAlavanca)) "0.000000, 0,90.000000" (Variables|Default|GetDelta) 2.0) false false)))

(event Input|KeyboardEvents|E
  (params (Key :type Key%20Structure :default "AnyKey"))
  (bind _ponte (Variables|Default|GetPonte))
  (bind _returnvalue (Transformation|GetActorRotation _ponte))
  (bind (_roll _pitch _yaw) (Math|Rotator|BreakRotator _returnvalue))
  (:Pressed
    (Variables|Default|SetPodeRodar true)
    (Transformation|SetActorRotation (Variables|Default|GetPonte) (Math|Rotator|MakeRotator 9e+01 _pitch _yaw))))

(fn ConstructionScript)