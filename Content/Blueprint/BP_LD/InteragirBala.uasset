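; InteragirBala is an interactable ammo pickup that adds bullets to the player's DoliosCharacter.
; Overlapping the Cube trigger enables input on the actor and shows a Billboard prompt; leaving disables input and hides it, without checking which actor overlapped.
; Pressing E adds BalasAumentadas to the character's Balas, then destroys the pickup if Destruir is set, otherwise it stays reusable.
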(event OnComponentBeginOverlap(Cube)
  (params (OverlappedComponent :type Primitive%20Component%20Object%20Reference) (OtherActor :type Actor%20Object%20Reference) (OtherComp :type Primitive%20Component%20Object%20Reference) (OtherBodyIndex :type Integer) (bFromSweep :type Boolean) (SweepResult :type Hit%20Result%20Structure%20%28by%20ref%29))
  ;[1 1 1] Interação trigger
  (Input|EnableInput (Game|GetPlayerController 0))
  (Development|SetHiddeninGame (Variables|Default|GetBillboard) false false))

(event OnComponentEndOverlap(Cube)
  (params (OverlappedComponent :type Primitive%20Component%20Object%20Reference) (OtherActor :type Actor%20Object%20Reference) (OtherComp :type Primitive%20Component%20Object%20Reference) (OtherBodyIndex :type Integer))
  ;[1 1 1] Interação trigger
  (Input|DisableInput (Game|GetPlayerController 0))
  (Development|SetHiddeninGame (Variables|Default|GetBillboard) true false))

(event Input|KeyboardEvents|E
  (params (Key :type Key%20Structure :default "AnyKey"))
  ;[1 1 1] Pegar Balas
  (:Pressed
    (bind _asdolios_character (Utilities|Casting|CastToDoliosCharacter (Game|GetPlayerCharacter 0)))
    (Variables|/Game/Blueprint/Character/DoliosCharacter.DoliosCharacter_C|SetBalas _asdolios_character (+ (Variables|/Game/Blueprint/Character/DoliosCharacter.DoliosCharacter_C|GetBalas _asdolios_character) (Variables|Default|GetBalasAumentadas)))
    (if (Variables|Default|GetDestruir)
      (Actor|DestroyActor))))

(fn ConstructionScript)