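; Gate actor (Portão) that the player opens by pressing E while holding a key.
; An overlap volume enables and disables the actor's input as things enter and leave, without filtering the overlapping actor.
; E checks the first entry of the DoliosCharacter's Chaves array, clears it and sets PodeRodar.
; Tick then smoothly interpolates the Billboard component's world rotation to zero; the UmaVez check does nothing.
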(event OnComponentBeginOverlap(Cube)
  (params (OverlappedComponent :type Primitive%20Component%20Object%20Reference) (OtherActor :type Actor%20Object%20Reference) (OtherComp :type Primitive%20Component%20Object%20Reference) (OtherBodyIndex :type Integer) (bFromSweep :type Boolean) (SweepResult :type Hit%20Result%20Structure%20%28by%20ref%29))
  (Input|EnableInput (Game|GetPlayerController 0)))

(event OnComponentEndOverlap(Cube)
  (params (OverlappedComponent :type Primitive%20Component%20Object%20Reference) (OtherActor :type Actor%20Object%20Reference) (OtherComp :type Primitive%20Component%20Object%20Reference) (OtherBodyIndex :type Integer))
  (Input|DisableInput (Game|GetPlayerController 0)))

(event EventTick
  (params (DeltaSeconds :type Float%20%28single-precision%29))
  (bind _billboard (Variables|Default|GetBillboard))
  (Variables|Default|SetDelta DeltaSeconds)
  (if (Variables|Default|GetPodeRodar)
    (Transformation|SetWorldRotation _billboard (Math|Interpolation|RInterpTo (Transformation|GetWorldRotation _billboard) "0,0.000000, 0" (Variables|Default|GetDelta) 2.0) false false)))

(event Input|KeyboardEvents|E
  (params (Key :type Key%20Structure :default "AnyKey"))
  (:Pressed
    (bind _asdolios_character (Utilities|Casting|CastToDoliosCharacter (Game|GetPlayerCharacter 0)))
    (if (Utilities|Array|Get(acopy) (Variables|/Game/Blueprint/Character/DoliosCharacter.DoliosCharacter_C|GetChaves _asdolios_character))
      (Variables|Default|SetPodeRodar true)
      (Utilities|Array|SetArrayElem (Variables|/Game/Blueprint/Character/DoliosCharacter.DoliosCharacter_C|GetChaves _asdolios_character) 0 false)
      (if (Variables|Default|GetUmaVez)
        _))))

(fn ConstructionScript)