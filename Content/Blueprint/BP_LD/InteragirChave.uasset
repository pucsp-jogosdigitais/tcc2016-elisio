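; Interactable key actor that grants the player a key, identified by IDChave.
; Overlapping the Cube enables input on the actor and shows a Billboard prompt, and leaving reverses both.
; Pressing E casts the player to DoliosCharacter and sets that index of its Chaves boolean array to true, resizing if needed.
; The actor then destroys itself if Destruir is set.
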(event OnComponentBeginOverlap(Cube)
  (params (OverlappedComponent :type Primitive%20Component%20Object%20Reference) (OtherActor :type Actor%20Object%20Reference) (OtherComp :type Primitive%20Component%20Object%20Reference) (OtherBodyIndex :type Integer) (bFromSweep :type Boolean) (SweepResult :type Hit%20Result%20Structure%20%28by%20ref%29))
  (Input|EnableInput (Game|GetPlayerController 0))
  (Development|SetHiddeninGame (Variables|Default|GetBillboard) false false))

(event OnComponentEndOverlap(Cube)
  (params (OverlappedComponent :type Primitive%20Component%20Object%20Reference) (OtherActor :type Actor%20Object%20Reference) (OtherComp :type Primitive%20Component%20Object%20Reference) (OtherBodyIndex :type Integer))
  (Input|DisableInput (Game|GetPlayerController 0))
  (Development|SetHiddeninGame (Variables|Default|GetBillboard) true false))

(event Collision|EventActorBeginOverlap
  (params (OtherActor :type Actor%20Object%20Reference)))

(event Input|KeyboardEvents|E
  (params (Key :type Key%20Structure :default "AnyKey"))
  (:Pressed
    (bind _asdolios_character (Utilities|Casting|CastToDoliosCharacter (Game|GetPlayerCharacter 0)))
    (Utilities|Array|SetArrayElem (Variables|/Game/Blueprint/Character/DoliosCharacter.DoliosCharacter_C|GetChaves _asdolios_character) (Variables|Default|GetIDChave) true true)
    (if (Variables|Default|GetDestruir)
      (Actor|DestroyActor))))

(fn ConstructionScript)