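; InformacoesTrigger is a level trigger that shows informational text to the player through DoliosCharacter.
; Overlapping the Trigger component enables input, makes the character's Visibilidade visible and sets Sinformacoes to the entry message; leaving disables input and hides it.
; Pressing E while input is enabled swaps the text to the interaction message.
; Overlap events act on player 0 without checking which actor overlapped.
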(event OnComponentBeginOverlap(Trigger)
  (params (OverlappedComponent :type Primitive%20Component%20Object%20Reference) (OtherActor :type Actor%20Object%20Reference) (OtherComp :type Primitive%20Component%20Object%20Reference) (OtherBodyIndex :type Integer) (bFromSweep :type Boolean) (SweepResult :type Hit%20Result%20Structure%20%28by%20ref%29))
  (Input|EnableInput (Game|GetPlayerController 0))
  (bind _asdolios_character (Utilities|Casting|CastToDoliosCharacter (Game|GetPlayerCharacter 0)))
  (Variables|/Game/Blueprint/Character/DoliosCharacter.DoliosCharacter_C|SetVisibilidade _asdolios_character "Visible")
  (Variables|/Game/Blueprint/Character/DoliosCharacter.DoliosCharacter_C|SetSinformacoes _asdolios_character (Variables|Default|GetInformaçãoQuandoEntra)))

(event OnComponentEndOverlap(Trigger)
  (params (OverlappedComponent :type Primitive%20Component%20Object%20Reference) (OtherActor :type Actor%20Object%20Reference) (OtherComp :type Primitive%20Component%20Object%20Reference) (OtherBodyIndex :type Integer))
  (Input|DisableInput (Game|GetPlayerController 0))
  (bind _asdolios_character (Utilities|Casting|CastToDoliosCharacter (Game|GetPlayerCharacter 0)))
  (Variables|/Game/Blueprint/Character/DoliosCharacter.DoliosCharacter_C|SetVisibilidade _asdolios_character "Hidden"))

(event EventBeginPlay)

(event Collision|EventActorBeginOverlap
  (params (OtherActor :type Actor%20Object%20Reference)))

(event EventTick
  (params (DeltaSeconds :type Float%20%28single-precision%29)))

(event Input|KeyboardEvents|E
  (params (Key :type Key%20Structure :default "AnyKey"))
  (:Pressed
    (bind _asdolios_character (Utilities|Casting|CastToDoliosCharacter (Game|GetPlayerCharacter 0)))
    (Variables|/Game/Blueprint/Character/DoliosCharacter.DoliosCharacter_C|SetSinformacoes _asdolios_character (Variables|Default|GetInformaçãoQuandoInteragi))))

(fn ConstructionScript)